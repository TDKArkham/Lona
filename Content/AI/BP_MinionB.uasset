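; BP_MinionB is a rat minion that knocks back characters touching its attack collision.
; The construction script snaps the attack collision component to the mesh's rat head socket.
; On overlap, any Character is launched horizontally away from the collision with a fixed upward lift, scaled by PushStrength and overriding its current velocity.
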(event `self.AttackCollison.OnComponentBeginOverlap`
  (params (OverlappedComponent :type "PrimitiveComponent Object Reference") (OtherActor :type "Actor Object Reference") (OtherComp :type "PrimitiveComponent Object Reference") (OtherBodyIndex :type Integer) (bFromSweep :type Boolean) (SweepResult :type "HitResult Structure (by ref)"))
  (bind _ascharacter (cast `Character` OtherActor))
  (bind (_returnvalue_x _returnvalue_y) (`KismetMathLibrary.BreakVector` (`KismetMathLibrary.GetDirectionUnitVector` (`SceneComponent.K2_GetComponentLocation` (`self.AttackCollison`)) (`self.K2_GetActorLocation` _ascharacter))))
  (bind (_returnvalue_x_2 _returnvalue_y_2) (`KismetMathLibrary.BreakVector` (`KismetMathLibrary.Normal` (`KismetMathLibrary.MakeVector` _returnvalue_x _returnvalue_y))))
  (`self.LaunchCharacter` _ascharacter (* (`KismetMathLibrary.MakeVector` _returnvalue_x_2 _returnvalue_y_2 0.3) (`self.PushStrength`)) true true))

(fn `UserConstructionScript`
  (`SceneComponent.K2_AttachToComponent` (`self.AttackCollison`) (`self.Mesh`) "Rat_HeadSocket" "SnapToTarget" "KeepRelative" "KeepWorld" false))