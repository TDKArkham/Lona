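; Level 1 boss that summons minions while the player's SideRunnerCharacter is inside its AttackTrigger.
; It plays a shaman attack montage and randomly spawns either a MinionA at one of the LocationsToGo points or a MinionB at Right, passing each its movement points.
; Only one minion is alive at a time; its OnDestroyed delegate clears the reference and spawns a replacement if the player is still in range.
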(event `self.AttackTrigger.OnComponentBeginOverlap`
  (params (OverlappedComponent :type "PrimitiveComponent Object Reference") (OtherActor :type "Actor Object Reference") (OtherComp :type "PrimitiveComponent Object Reference") (OtherBodyIndex :type Integer) (bFromSweep :type Boolean) (SweepResult :type "HitResult Structure (by ref)"))
  (cast `SideRunnerCharacter` OtherActor)
  (set `self.bIsInAttackRange` true)
  (`self.SpawnMinion`))

(event `self.AttackTrigger.OnComponentEndOverlap`
  (params (OverlappedComponent :type "PrimitiveComponent Object Reference") (OtherActor :type "Actor Object Reference") (OtherComp :type "PrimitiveComponent Object Reference") (OtherBodyIndex :type Integer))
  (cast `SideRunnerCharacter` OtherActor)
  (set `self.bIsInAttackRange` false))

(event `SpawnMinion`
  (bind _locationstogo (`self.LocationsToGo`))
  (`self.MinionA`
    (:`then`)
    (:`else`
      (`self.MinionB`
        (:`then`)
        (:`else`
          (if (`self.bIsInAttackRange`)
            (`self.PlayAnimMontage` "/Game/Shaman/Animations/A_shaman__shaman_attack_Montage.A_shaman__shaman_attack_Montage")
            (switch `int` (`KismetMathLibrary.RandomIntegerInRange` 0 1)
              (:`0`
                (bind _returnvalue (`|SpawnActorFromClass` "/Game/AI/BP_MinionA.BP_MinionA_C" (`KismetMathLibrary.MakeTransform` (`|GetArrayItem` _locationstogo (`KismetMathLibrary.RandomIntegerInRange` 0 (- (`KismetArrayLibrary.Array_Length` _locationstogo) 1))) (struct :`Yaw` 90.0)) "AlwaysSpawn" "OverrideRootScale" null _locationstogo null))
                (bind _output_get (set `self.MinionA` _returnvalue))
                (add `self.OnDestroyed` _output_get (delegate `OnDestroyed_MinionA`)))
              (:`1`
                (bind _returnvalue_2 (`|SpawnActorFromClass` :`Class` "/Game/AI/BP_MinionB.BP_MinionB_C" :`SpawnTransform` (`KismetMathLibrary.MakeTransform` (`self.Right`)) :`CollisionHandlingOverride` "AlwaysSpawn" :`TransformScaleMethod` "OverrideRootScale" :`Left` (`self.Left`) :`Right` (`self.Right`) :`Instigator` null))
                (bind _output_get_2 (set `self.MinionB` _returnvalue_2))
                (add `self.OnDestroyed` _output_get_2 (delegate `OnDestroyed_MinionB`))))))))))

(event `OnDestroyed_MinionA` :!signature `self.OnDestroyed`
  (params (DestroyedActor :type "Actor Object Reference"))
  (set `self.MinionA` null)
  (`self.SpawnMinion`))

(event `OnDestroyed_MinionB` :!signature `self.OnDestroyed`
  (params (DestroyedActor :type "Actor Object Reference"))
  (set `self.MinionB` null)
  (`self.SpawnMinion`))

(fn `UserConstructionScript`)