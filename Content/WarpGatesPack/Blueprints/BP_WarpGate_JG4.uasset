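; Warp gate actor (JG4 variant) that switches an animated warp effect on and off.
; Construction script builds dynamic materials for gate, ring, selectable plane and flow, applying color, gate hue shift and initial on/off state.
; Activate and Deactivate events play or reverse a timeline driving material parameters, flow length and ring spin, reversing from the end on first deactivation if starting on.
; Tick rotates gate and ring independently.
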(event `self.ReceiveBeginPlay`
  (set `self.StartWarp_On` (`self.WarpGate_On`)))

(event `Activate_Warp`
  (bind _warp_on (`self.Warp_On`))
  ;[1 1 1] Warp Activate / Deactivate
  (set `self.WarpGate_On` true)
  (bind (_direction _warp_on_2 _ring _warpflow) (`Timeline|Timeline_Warp` :!label _label)
    (:`Update`
      (set `self.Warp_On` _warp_on_2)
      (set `self.RingRotationRate` _ring)
      (`SceneComponent.SetRelativeScale3D` (`self.SM_WarpFlow`) (`KismetMathLibrary.MakeVector` 1.0 (`KismetMathLibrary.Lerp` 0.2 (`self.WarpFlow_Length`) _warpflow) 1.0))
      (`MaterialInstanceDynamic.SetScalarParameterValue` (`self.MID_WarpFlow`) "Warp_On" _warpflow)
      (`MaterialInstanceDynamic.SetScalarParameterValue` (`self.MID_Ring_JG4`) "Warp_On" (`self.RingRotationRate`))
      (`MaterialInstanceDynamic.SetScalarParameterValue` (`self.MID_WarpPlane`) "Warp_On" _warp_on)
      (`MaterialInstanceDynamic.SetScalarParameterValue` (`self.MID_WarpGate_JG4`) "Warp_On" _warp_on)
      (`MaterialInstanceDynamic.SetScalarParameterValue` (`self.MID_WarpFlow`) "Wave_2_UV" (`KismetMathLibrary.SelectFloat` (`KismetMathLibrary.Lerp` 1.0 0.0 _warp_on) (`KismetMathLibrary.Lerp` 0.0 1.0 _warp_on) (`self.Swirling`))))))

(event `Deactivate_Warp`
  ;[1 1 1] Warp Activate / Deactivate
  (set `self.WarpGate_On` false)
  (if (`self.StartWarp_On`)
    (set `self.StartWarp_On` false)
    (goto _label :!via `ReverseFromEnd`)
    (else
      (goto _label :!via `Reverse`))))

(event `self.ReceiveTick`
  (params (DeltaSeconds :type "Float (single-precision)"))
  (bind _rotationrate (`self.RotationRate`))
  (bind _returnvalue (* (`self.RingRotationRate`) -1.0))
  ;[1 1 1] Ring Rotation
  (if (!= _rotationrate 0.0)
    (`SceneComponent.K2_AddLocalRotation` (`self.SM_Warpgate`) (`KismetMathLibrary.MakeRotator` 0.0 (* _rotationrate 0.1)) false false))
  (if (!= _returnvalue 0.0)
    (`SceneComponent.K2_AddLocalRotation` (`self.SM_Warpgate_JG4_Ring`) (`KismetMathLibrary.MakeRotator` 0.0 _returnvalue) false false)))

(fn `UserConstructionScript`
  (bind _warp_on (`self.Warp_On`))
  (switch `int` (`self.WarpPlane_Type`)
    (:`Default`
      (bind _returnvalue (`KismetMaterialLibrary.CreateDynamicMaterialInstance` "/Game/WarpGatesPack/Materials/WarpGate_JG4/MI_WarpPlane_A_JG4.MI_WarpPlane_A_JG4" :!label _label))
      (set `self.MID_WarpPlane` _returnvalue))
    (:`0`
      (goto _label))
    (:`1`
      (bind _returnvalue_2 (`KismetMaterialLibrary.CreateDynamicMaterialInstance` "/Game/WarpGatesPack/Materials/WarpGate_JG4/MI_WarpPlane_B_JG4.MI_WarpPlane_B_JG4"))
      (set `self.MID_WarpPlane` _returnvalue_2))
    (:`2`
      (bind _returnvalue_3 (`KismetMaterialLibrary.CreateDynamicMaterialInstance` "/Game/WarpGatesPack/Materials/WarpGate_JG4/MI_WarpPlane_C_JG4.MI_WarpPlane_C_JG4"))
      (set `self.MID_WarpPlane` _returnvalue_3))
    (:`3`
      (bind _returnvalue_4 (`KismetMaterialLibrary.CreateDynamicMaterialInstance` "/Game/WarpGatesPack/Materials/WarpGate_JG4/MI_WarpPlane_D_JG4.MI_WarpPlane_D_JG4"))
      (set `self.MID_WarpPlane` _returnvalue_4)))
  (`PrimitiveComponent.SetMaterial` (`self.SM_WarpPlane`) 0 (`self.MID_WarpPlane`))
  (bind _returnvalue_5 (`KismetMaterialLibrary.CreateDynamicMaterialInstance` "/Game/WarpGatesPack/Materials/WarpGate_JG4/MI_WarpGate_JG4.MI_WarpGate_JG4"))
  (bind _output_get (set `self.MID_WarpGate_JG4` _returnvalue_5))
  (`PrimitiveComponent.SetMaterial` (`self.SM_Warpgate`) 0 _output_get)
  (`MaterialInstanceDynamic.SetScalarParameterValue` _output_get "HueShift" (`self.HueShift`))
  (bind _returnvalue_6 (`KismetMaterialLibrary.CreateDynamicMaterialInstance` "/Game/WarpGatesPack/Materials/WarpGate_JG4/MI_WarpGate_JG4_Ring.MI_WarpGate_JG4_Ring"))
  (bind _output_get_2 (set `self.MID_Ring_JG4` _returnvalue_6))
  (`PrimitiveComponent.SetMaterial` (`self.SM_Warpgate_JG4_Ring`) 0 _output_get_2)
  (switch `int` (`self.WarpFlow_Type`)
    (:`Default`
      (bind _returnvalue_7 (`KismetMaterialLibrary.CreateDynamicMaterialInstance` "/Game/WarpGatesPack/Materials/WarpEnergy/MI_WarpFlow_A.MI_WarpFlow_A" :!label _label_2))
      (set `self.MID_WarpFlow` _returnvalue_7))
    (:`0`
      (goto _label_2))
    (:`1`
      (bind _returnvalue_8 (`KismetMaterialLibrary.CreateDynamicMaterialInstance` "/Game/WarpGatesPack/Materials/WarpEnergy/MI_WarpFlow_B.MI_WarpFlow_B"))
      (set `self.MID_WarpFlow` _returnvalue_8))
    (:`2`
      (bind _returnvalue_9 (`KismetMaterialLibrary.CreateDynamicMaterialInstance` "/Game/WarpGatesPack/Materials/WarpEnergy/MI_WarpFlow_C.MI_WarpFlow_C"))
      (set `self.MID_WarpFlow` _returnvalue_9))
    (:`3`
      (bind _returnvalue_10 (`KismetMaterialLibrary.CreateDynamicMaterialInstance` "/Game/WarpGatesPack/Materials/WarpEnergy/MI_WarpFlow_D.MI_WarpFlow_D"))
      (set `self.MID_WarpFlow` _returnvalue_10)))
  (`PrimitiveComponent.SetMaterial` (`self.SM_WarpFlow`) 0 (`self.MID_WarpFlow`))
  (if (`self.WarpGate_On`)
    (set `self.Warp_On` 1.0)
    (else
      (set `self.Warp_On` 0.0)))
  (`MaterialInstanceDynamic.SetScalarParameterValue` (`self.MID_WarpPlane`) "Warp_On" _warp_on)
  (`MaterialInstanceDynamic.SetScalarParameterValue` (`self.MID_WarpGate_JG4`) "Warp_On" _warp_on)
  (`MaterialInstanceDynamic.SetScalarParameterValue` (`self.MID_Ring_JG4`) "Warp_On" _warp_on)
  (`MaterialInstanceDynamic.SetScalarParameterValue` (`self.MID_WarpFlow`) "Warp_On" _warp_on)
  (set `self.RingRotationRate` _warp_on)
  (`SceneComponent.SetRelativeScale3D` (`self.SM_WarpFlow`) (`KismetMathLibrary.MakeVector` 1.0 (`KismetMathLibrary.Lerp` 0.2 (`self.WarpFlow_Length`) _warp_on) 1.0))
  (`MaterialInstanceDynamic.SetVectorParameterValue` (`self.MID_WarpPlane`) "WarpColor" (`self.WarpColor`))
  (`MaterialInstanceDynamic.SetVectorParameterValue` (`self.MID_WarpGate_JG4`) "WarpColor" (`self.WarpColor`))
  (`MaterialInstanceDynamic.SetVectorParameterValue` (`self.MID_Ring_JG4`) "WarpColor" (`self.WarpColor`))
  (`MaterialInstanceDynamic.SetVectorParameterValue` (`self.MID_WarpFlow`) "WarpColor" (`self.WarpColor`)))