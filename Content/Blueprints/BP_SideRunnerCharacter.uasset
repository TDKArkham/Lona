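; Side runner character Blueprint that reacts to damage and keeps its hair mesh animated with the body.
; On BeginPlay it binds to the AttributeComponent's health change, and on a negative delta prints a debug hurt message.
; The same event writes the current time to the mesh materials' TimeToHit parameter, leaving any hit effect to the shader.
; The construction script sets Mesh as the hair's master pose component.
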(event `self.ReceiveBeginPlay`
  (add `SRAttributeComponent.OnHealthChanged` (`self.AttributeComponent`) (delegate `OnHealthChanged_Event`)))

(event `OnHealthChanged_Event`
  (params (InstigateActor :type "Actor Object Reference") (OwnerComponent :type "SRAttributeComponent Object Reference") (NewValue :type "Float (single-precision)") (Delta :type "Float (single-precision)"))
  (if (< Delta 0.0)
    (`MeshComponent.SetScalarParameterValueOnMaterials` (`self.Mesh`) "TimeToHit" (`GameplayStatics.GetTimeSeconds`))
    (`KismetSystemLibrary.PrintString` "Got Hurt !!!" true false (struct :`R` 1.0 :`G` 0.454242 :`B` 0.574677 :`A` 1.0) 5.0)))

(fn `UserConstructionScript`
  (`SkinnedMeshComponent.SetLeaderPoseComponent` (`self.HairS2`) (`self.Mesh`) false))