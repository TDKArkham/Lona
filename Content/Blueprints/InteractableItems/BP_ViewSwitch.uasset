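; BP_ViewSwitch is a one-shot trigger box that plays a camera tour of a mechanism and its switch when a SideRunnerCharacter enters it.
; On overlap it disables its collision, then, if both targets are valid, locks player input and blends the view to TargetMechanism, then TargetSwitch, pausing at each.
; The view then blends back to the character over SwitchBlendTime minus MechanismBlendTime, and input is restored.
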(event `self.BoxCollision.OnComponentBeginOverlap`
  (params (OverlappedComponent :type "PrimitiveComponent Object Reference") (OtherActor :type "Actor Object Reference") (OtherComp :type "PrimitiveComponent Object Reference") (OtherBodyIndex :type Integer) (bFromSweep :type Boolean) (SweepResult :type "HitResult Structure (by ref)"))
  (bind _returnvalue (`GameplayStatics.GetPlayerController` 0))
  (bind _mechanismblendtime (`self.MechanismBlendTime`))
  (bind _switchblendtime (`self.SwitchBlendTime`))
  (bind _returnvalue_2 (- (`self.SwitchBlendTime`) (`self.MechanismBlendTime`)))
  (bind _asside_runner_character (cast `SideRunnerCharacter` OtherActor))
  (`PrimitiveComponent.SetCollisionEnabled` (`self.BoxCollision`) "NoCollision")
  (if (and (`KismetSystemLibrary.IsValid` (`self.TargetMechanism`)) (`KismetSystemLibrary.IsValid` (`self.TargetSwitch`)))
    (`self.DisableInput` _asside_runner_character _returnvalue)
    (`PlayerController.SetViewTargetWithBlend` _returnvalue (`self.TargetMechanism`) _mechanismblendtime "VTBlend_Linear" 0.0 false)
    (`KismetSystemLibrary.Delay` _mechanismblendtime)
    (`KismetSystemLibrary.Delay` (`self.MechanismStayTime`))
    (`PlayerController.SetViewTargetWithBlend` _returnvalue (`self.TargetSwitch`) _switchblendtime "VTBlend_Linear" 0.0 false)
    (`KismetSystemLibrary.Delay` _switchblendtime)
    (`KismetSystemLibrary.Delay` (`self.SwitchStayTime`))
    (`PlayerController.SetViewTargetWithBlend` _returnvalue _asside_runner_character _returnvalue_2 "VTBlend_Linear" 0.0 false)
    (`KismetSystemLibrary.Delay` _returnvalue_2)
    (`self.EnableInput` _asside_runner_character _returnvalue)))

(fn `UserConstructionScript`)