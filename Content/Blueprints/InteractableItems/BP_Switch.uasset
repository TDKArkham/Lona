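; BP_Switch is a one-shot interactable switch that the player triggers with a projectile.
; An overlap on OpenTrigger from a BP_PlayerProjectile disables the trigger's collision and, if TargetActor is valid, sends it InteractMessage.
; The PullRod timeline then animates the Scene component's roll toward TargetRotation while keeping pitch and yaw.
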(event `self.OpenTrigger.OnComponentBeginOverlap`
  (params (OverlappedComponent :type "PrimitiveComponent Object Reference") (OtherActor :type "Actor Object Reference") (OtherComp :type "PrimitiveComponent Object Reference") (OtherBodyIndex :type Integer) (bFromSweep :type Boolean) (SweepResult :type "HitResult Structure (by ref)"))
  (bind _scene (`self.Scene`))
  (bind (_relativerotation_roll _relativerotation_pitch _relativerotation_yaw) (`KismetMathLibrary.BreakRotator` (`SceneComponent.RelativeRotation` _scene)))
  (cast `/Game/Blueprints/BP_PlayerProjectile` OtherActor)
  (`PrimitiveComponent.SetCollisionEnabled` (`self.OpenTrigger`) "NoCollision")
  (bind _targetactor (`self.TargetActor`)
    (:`then`
      (message `SRInteractInterface.Interact` _targetactor)
      (bind (_direction _pullrate) (`Timeline|PullRod`)
        (:`Update`
          (`SceneComponent.K2_SetRelativeRotation` _scene (`KismetMathLibrary.MakeRotator` (* _pullrate (`self.TargetRotation`)) _relativerotation_pitch _relativerotation_yaw) false false))))
    (:`else`)))

(fn `UserConstructionScript`)