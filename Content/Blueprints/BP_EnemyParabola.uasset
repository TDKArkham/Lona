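; BP_EnemyParabola is an enemy actor that flies in an arc from its spawn point toward a target, then explodes.
; On BeginPlay it records its own and the target's locations once, so it does not track later movement.
; A timeline lerps horizontal position along one track and adds a height offset scaled by FlyHeight from another.
; When the timeline finishes it calls HitExplode; movement is unswept.
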(event `self.ReceiveBeginPlay`
  (bind (_startlocation_x _startlocation_y _startlocation_z) (`KismetMathLibrary.BreakVector` (`self.StartLocation`)))
  (bind (_targetlocation_x _targetlocation_y _targetlocation_z) (`KismetMathLibrary.BreakVector` (`self.TargetLocation`)))
  (set `self.StartLocation` (`self.K2_GetActorLocation`))
  (set `self.TargetLocation` (`self.K2_GetActorLocation` (`self.Target`)))
  (bind (_direction _xy_track _z_track) (`Timeline|Timeline_0`)
    (:`Update`
      (bind _returnvalue (* _z_track (`self.FlyHeight`)))
      (`self.K2_SetActorLocation` (`KismetMathLibrary.VLerp` (`KismetMathLibrary.MakeVector` _startlocation_x _startlocation_y (+ _returnvalue _startlocation_z)) (`KismetMathLibrary.MakeVector` _targetlocation_x _targetlocation_y (+ _returnvalue _targetlocation_z)) _xy_track)))
    (:`Finished`
      (`self.HitExplode`))))

(fn `UserConstructionScript`)