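; Player controller that owns the game's UI flow between main menu, HUD and in-game pause menu.
; On begin play it shows the main menu with UI-only input and a visible cursor.
; BeginClicked removes that menu, waits out a camera blend delay, then adds the HUD and marks the game as begun.
; Once begun, Escape toggles the pause menu, switching pause state, input mode and cursor.
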(event `self.ReceiveBeginPlay`
  (bind _returnvalue (`GameplayStatics.GetPlayerController` 0))
  (bind _returnvalue_2 (`|CreateWidget` "/Game/UI/WBP_MainMenu.WBP_MainMenu_C"))
  (bind _output_get (set `self.MainMenuWidget` _returnvalue_2))
  (`UserWidget.AddToViewport` _output_get 0)
  (`WidgetBlueprintLibrary.SetInputMode_UIOnlyEx` _returnvalue _returnvalue_2)
  (set `PlayerController.bShowMouseCursor` true _returnvalue))

(event `/Game/Blueprints/BP_BeginPlay_Interface.BeginClicked`
  (params (CameraBlendTime :type "Float (double-precision)"))
  (`Widget.RemoveFromParent` (`self.MainMenuWidget`))
  (`KismetSystemLibrary.Delay` CameraBlendTime)
  (bind _returnvalue (`|CreateWidget` "/Game/UI/WBP_MainHUD.WBP_MainHUD_C"))
  (`UserWidget.AddToViewport` _returnvalue 0)
  (set `self.bIsGameBegin` true))

(event `Key|Escape` :paused true
  (params (Key :type "Key Structure"))
  (bind _returnvalue (`GameplayStatics.GetPlayerController` 0))
  (bind _returnvalue_2 (`GameplayStatics.GetPlayerController` 0))
  (:`Pressed`
    (if (`self.bIsGameBegin`)
      (`self.InGameMenu`
        (:`then`
          (`GameplayStatics.SetGamePaused` false)
          (`Widget.RemoveFromParent` (`self.InGameMenu`))
          (set `self.InGameMenu` null)
          (`WidgetBlueprintLibrary.SetInputMode_GameOnly` _returnvalue)
          (set `PlayerController.bShowMouseCursor` false _returnvalue))
        (:`else`
          (`GameplayStatics.SetGamePaused` true)
          (bind _returnvalue_3 (`|CreateWidget` "/Game/UI/WBP_InGameMenu.WBP_InGameMenu_C"))
          (bind _output_get (set `self.InGameMenu` _returnvalue_3))
          (`UserWidget.AddToViewport` _output_get 0)
          (`WidgetBlueprintLibrary.SetInputMode_GameAndUIEx` _returnvalue_2 _output_get "DoNotLock" false)
          (set `PlayerController.bShowMouseCursor` true _returnvalue_2))))))

(fn `UserConstructionScript`)